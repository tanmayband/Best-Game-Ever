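; BP_MapNode is a map node actor that swaps its mesh material to show hover and activation state.
; It extends parent hover and activation logic, changing the material on hover start and stop only when the parent call returns true.
; Hover uses an emissive material, activation uses a separate emissive instance, and both hover stop and deactivation restore the basic material.
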(event EventBeginPlay)

(event Collision|EventActorBeginOverlap
  (params (OtherActor :type Actor%20Object%20Reference)))

(event EventTick
  (params (DeltaSeconds :type Float%20%28single-precision%29)))

(event EventToggleActivate
  (params (activate :type Boolean))
  (|CallParentFunction activate)
  (Rendering|Material|SetMaterial (Variables|Character|GetMesh) 0 (select activate "/Game/Materials/Test/MI_Emissive_1.MI_Emissive_1" "/Game/Materials/Test/M_Basic.M_Basic")))

(fn ConstructionScript)

(fn OnMouseHoverStop
  (bind _returnvalue (|CallParentFunction))
  (if _returnvalue
    (Rendering|Material|SetMaterial (Variables|Character|GetMesh) 0 "/Game/Materials/Test/M_Basic.M_Basic"))
  (return _returnvalue))

(fn OnMouseHover
  (bind _returnvalue (|CallParentFunction))
  (if _returnvalue
    (Rendering|Material|SetMaterial (Variables|Character|GetMesh) 0 "/Game/Materials/Test/M_Emissive.M_Emissive"))
  (return _returnvalue))